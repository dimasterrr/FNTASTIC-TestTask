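; AI controller for turtle pawns that starts their behavior tree when possessed.
; On possess, it casts the pawn to TurtlePawn, runs BT_Turtle, then seeds the blackboard with the pawn's movement mode, start location and end location.
; Movement settings come from each pawn, while the controller only hands them to the tree.
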(event `self.ReceivePossess`
  (params (PossessedPawn :type "Pawn Object Reference"))
  (bind _asturtle_pawn (cast `TurtlePawn` PossessedPawn))
  (`self.RunBehaviorTree` "/Game/Blueprints/Controllers/BehaviorTree/BT_Turtle.BT_Turtle")
  (`BlackboardComponent.SetValueAsEnum` (`AIBlueprintHelperLibrary.GetBlackboard` null) "MovementMode" (`TurtlePawn.GetMovementMode` _asturtle_pawn))
  (`BlackboardComponent.SetValueAsVector` (`AIBlueprintHelperLibrary.GetBlackboard` null) "StartLocation" (`TurtlePawn.GetStartLocation` _asturtle_pawn))
  (`BlackboardComponent.SetValueAsVector` (`AIBlueprintHelperLibrary.GetBlackboard` null) "EndLocation" (`TurtlePawn.GetEndLocation` _asturtle_pawn)))

(fn `UserConstructionScript`)